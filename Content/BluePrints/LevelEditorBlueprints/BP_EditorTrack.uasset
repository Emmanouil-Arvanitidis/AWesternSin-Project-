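; BP_EditorTrack is a numbered track piece for the level editor that can rotate in response to events.
; RotateTrack acts only on a matching TrackNo, playing a timeline forward from zero yaw or in reverse otherwise to animate relative yaw.
; Separate editor events reassign the track's ID and snap the tile a quarter turn about yaw.
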(event `/Game/BluePrints/BlueprintInterfaces/BPI_LeverFunctionality.RotateTrack`
  (params (TrackNumber :type Integer))
  (bind (_returnvalue_roll _returnvalue_pitch _returnvalue_yaw) (`KismetMathLibrary.BreakRotator` (`self.K2_GetActorRotation`)))
  (if (== TrackNumber (`self.TrackNo`))
    (if (== _returnvalue_yaw 0.0)
      (bind (_direction _newtrack_0) (`Timeline|Timeline` :!via `PlayFromStart` :!label _label)
        (:`Update`
          (`self.K2_SetActorRelativeRotation` (`KismetMathLibrary.MakeRotator` 0.0 0.0 _newtrack_0))))
      (else
        (goto _label :!via `ReverseFromEnd`)))))

(event `/Game/BluePrints/LevelEditorBlueprints/Interfaces/BPI_TileFunctionality.ChangeID(Editor)`
  (params (`New ID` :type Integer))
  (set `self.TrackNo` `New ID`))

(event `/Game/BluePrints/LevelEditorBlueprints/Interfaces/BPI_TileFunctionality.RotateTile(Editor)`
  (bind (_returnvalue_roll _returnvalue_pitch _returnvalue_yaw) (`KismetMathLibrary.BreakRotator` (`self.K2_GetActorRotation`)))
  (`self.K2_SetActorRotation` (`KismetMathLibrary.MakeRotator` _returnvalue_roll _returnvalue_pitch (+ _returnvalue_yaw 90.0))))

(fn `UserConstructionScript`)