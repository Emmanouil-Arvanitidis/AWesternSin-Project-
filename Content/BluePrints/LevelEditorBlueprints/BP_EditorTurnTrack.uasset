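; Turnable track piece for the level editor that rotates in yaw when triggered by its track ID.
; RotateTrack compares the incoming number to TurnTrackID and, on a match, plays a timeline that adds its value to the stored CurrentRotation.
; CurrentRotation is captured at BeginPlay and after each timeline finishes, so turns accumulate.
; Editor events reassign the ID or turn the tile by a quarter turn, also updating the stored rotation.
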(event `self.ReceiveBeginPlay`
  (bind (_returnvalue_roll _returnvalue_pitch _returnvalue_yaw) (`KismetMathLibrary.BreakRotator` (`self.K2_GetActorRotation`)))
  (set `self.CurrentRotation` _returnvalue_yaw))

(event `/Game/BluePrints/BlueprintInterfaces/BPI_LeverFunctionality.RotateTrack`
  (params (TrackNumber :type Integer))
  (bind (_returnvalue_roll _returnvalue_pitch _returnvalue_yaw) (`KismetMathLibrary.BreakRotator` (`self.K2_GetActorRotation`)))
  (if (== TrackNumber (`self.TurnTrackID`))
    (bind (_direction _newtrack_0) (`Timeline|Timeline` :!via `PlayFromStart`)
      (:`Update`
        (`self.K2_SetActorRotation` (`KismetMathLibrary.MakeRotator` 0.0 0.0 (+ _newtrack_0 (`self.CurrentRotation`)))))
      (:`Finished`
        (set `self.CurrentRotation` _returnvalue_yaw)))))

(event `/Game/BluePrints/LevelEditorBlueprints/Interfaces/BPI_TileFunctionality.ChangeID(Editor)`
  (params (`New ID` :type Integer))
  (set `self.TurnTrackID` `New ID`))

(event `/Game/BluePrints/LevelEditorBlueprints/Interfaces/BPI_TileFunctionality.RotateTile(Editor)`
  (bind (_returnvalue_roll _returnvalue_pitch _returnvalue_yaw) (`KismetMathLibrary.BreakRotator` (`self.K2_GetActorRotation`)))
  (bind _returnvalue (+ _returnvalue_yaw 90.0))
  (`self.K2_SetActorRotation` (`KismetMathLibrary.MakeRotator` _returnvalue_roll _returnvalue_pitch _returnvalue))
  (set `self.CurrentRotation` _returnvalue))

(fn `UserConstructionScript`)