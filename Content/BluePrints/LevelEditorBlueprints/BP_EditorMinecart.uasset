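; Level-editor minecart that, when RotateTrack is called with its CartID, travels tile by tile along track splines.
; MoveCart takes the last overlapping straight track, else turn track, and CheckRotationRelationship tests yaw alignment.
; Timelines drive it along the spline forward or reversed by entry facing, then call MoveCart again, resetting to its origin after a delay when blocked.
; Editor events set ID and rotation; touching explosion beams only plays a sound.
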(event `self.ReceiveBeginPlay`
  ; Origin Variables are set so that the Cart knows where to reset to
  (set `self.Origin Location` (`SceneComponent.K2_GetComponentLocation` (`self.Cube`)))
  (set `self.Origin Rotation` (`SceneComponent.K2_GetComponentRotation` (`self.Cube`))))

(event `Reset Cart`
  ; Called when cart cannot move to new track
  (`KismetSystemLibrary.Delay` 1.0)
  (`SceneComponent.K2_SetWorldLocationAndRotation` (`self.Cube`) (`self.Origin Location`) (`self.Origin Rotation`) false false))

(event `/Game/BluePrints/BlueprintInterfaces/BPI_LeverFunctionality.RotateTrack`
  (params (TrackNumber :type Integer))
  ; Calls MoveCart event if ID is correct
  (if (== TrackNumber (`self.CartID`))
    (`self.MoveCart`)))

(event `self.Box.OnComponentBeginOverlap`
  (params (OverlappedComponent :type "PrimitiveComponent Object Reference") (OtherActor :type "Actor Object Reference") (OtherComp :type "PrimitiveComponent Object Reference") (OtherBodyIndex :type Integer) (bFromSweep :type Boolean) (SweepResult :type "HitResult Structure (by ref)"))
  (cast `/Game/BluePrints/BaseGameBlueprints/BP_ExplotionBeams` OtherActor)
  (`GameplayStatics.PlaySound2D` "/Game/TemplateFolders/StarterContent/Audio/Explosion01.Explosion01" 1.0 1.0 0.0 null null))

(event `MoveCart`
  (bind _overlappingactors (`PrimitiveComponent.GetOverlappingActors` (`self.Box`) "/Game/BluePrints/LevelEditorBlueprints/BP_EditorTrack.BP_EditorTrack_C"))
  (bind _overlappingactors_2 (`PrimitiveComponent.GetOverlappingActors` (`self.Box`) "/Game/BluePrints/LevelEditorBlueprints/BP_EditorTurnTrack.BP_EditorTurnTrack_C"))
  (bind _output (`|GetArrayItem` _overlappingactors_2 (- (`KismetArrayLibrary.Array_Length` _overlappingactors_2) 1)))
  (bind _output_2 (`|GetArrayItem` _overlappingactors (- (`KismetArrayLibrary.Array_Length` _overlappingactors) 1)))
  ; Cart Pathfinding Logic
  (`/Engine/EditorBlueprintResources/StandardMacros.IsValid` _output_2
    (:`Is Valid`
      (`self.CheckRotationRelationship` true _output_2))
    (:`Is Not Valid`
      (`/Engine/EditorBlueprintResources/StandardMacros.IsValid` _output
        (:`Is Valid`
          (`self.CheckRotationRelationship` false _output))
        (:`Is Not Valid`
          (`self.Reset Cart`))))))

(event `Move along Straight Path`
  (params (SplineRef :type "SplineComponent Object Reference"))
  ; Cart Pathfinding Logic
  (bind _output_get (set `self.Spline Ref` SplineRef))
  (if (== (`self.K2_GetActorRotation` (`ActorComponent.GetOwner` _output_get)) (`SceneComponent.K2_GetComponentRotation` (`self.Cube`)) :`ErrorTolerance` 10.0)
    (bind (_direction _newtrack_1) (`Timeline|MoveAlongSpline` :!via `PlayFromStart`)
      (:`Update`
        (`SceneComponent.K2_SetWorldLocation` (`self.Cube`) (`SplineComponent.GetLocationAtDistanceAlongSpline` (`self.Spline Ref`) (`KismetMathLibrary.Lerp` 0.0 (`SplineComponent.GetSplineLength` (`self.Spline Ref`)) _newtrack_1) "World") false false))
      (:`Finished`
        (`self.MoveCart`)))
    (else
      (bind (_direction_2 _newtrack_1_2) (`Timeline|MoveAlongSplineCopy` :!via `PlayFromStart`)
        (:`Update`
          (`SceneComponent.K2_SetWorldLocation` (`self.Cube`) (`SplineComponent.GetLocationAtDistanceAlongSpline` (`self.Spline Ref`) (`KismetMathLibrary.Lerp` (`SplineComponent.GetSplineLength` (`self.Spline Ref`)) 0.0 _newtrack_1_2) "World") false false))
        (:`Finished`
          (`self.MoveCart`))))))

(event `Move Along Turn Track`
  (params (SplineRef :type "SplineComponent Object Reference"))
  (bind _spline_ref (`self.Spline Ref`))
  (bind _spline_ref_2 (`self.Spline Ref`))
  (bind _returnvalue (`SplineComponent.GetSplineLength` (`self.Spline Ref`)))
  ; Cart Pathfinding Logic
  (bind _output_get (set `self.Spline Ref` SplineRef))
  (if (== (`self.K2_GetActorRotation` (`ActorComponent.GetOwner` _output_get)) (`SceneComponent.K2_GetComponentRotation` (`self.Cube`)) :`ErrorTolerance` 10.0)
    (bind (_direction _newtrack_1) (`Timeline|0-1` :!via `PlayFromStart`)
      (:`Update`
        (bind _returnvalue_2 (`KismetMathLibrary.Lerp` 0.0 (`SplineComponent.GetSplineLength` (`self.Spline Ref`)) _newtrack_1))
        (`SceneComponent.K2_SetWorldLocationAndRotation` (`self.Cube`) (`SplineComponent.GetLocationAtDistanceAlongSpline` _spline_ref _returnvalue_2 "World") (`SplineComponent.GetRotationAtDistanceAlongSpline` _spline_ref _returnvalue_2 "World") false false))
      (:`Finished`
        (`self.MoveCart`)))
    (else
      (bind (_direction_2 _newtrack_1_2) (`Timeline|Timeline` :!via `PlayFromStart`)
        (:`Update`
          (bind (_returnvalue_roll _returnvalue_pitch _returnvalue_yaw) (`KismetMathLibrary.BreakRotator` (`SplineComponent.GetRotationAtDistanceAlongSpline` _spline_ref_2 (`KismetMathLibrary.Lerp` _returnvalue 0.0 _newtrack_1_2) "World")))
          (`SceneComponent.K2_SetWorldLocationAndRotation` (`self.Cube`) (`SplineComponent.GetLocationAtDistanceAlongSpline` _spline_ref_2 (`KismetMathLibrary.Lerp` _returnvalue 0.0 _newtrack_1_2) "World") (`KismetMathLibrary.MakeRotator` _returnvalue_roll _returnvalue_pitch (- _returnvalue_yaw 180.0)) false false))
        (:`Finished`
          (`self.MoveCart`))))))

(event `/Game/BluePrints/LevelEditorBlueprints/Interfaces/BPI_TileFunctionality.ChangeID(Editor)`
  (params (`New ID` :type Integer))
  ; Level Editor Funcitons
  (set `self.CartID` `New ID`))

(event `/Game/BluePrints/LevelEditorBlueprints/Interfaces/BPI_TileFunctionality.RotateTile(Editor)`
  (bind (_returnvalue_roll _returnvalue_pitch _returnvalue_yaw) (`KismetMathLibrary.BreakRotator` (`SceneComponent.K2_GetComponentRotation` (`self.Cube`))))
  (bind _returnvalue (`KismetMathLibrary.MakeRotator` _returnvalue_roll _returnvalue_pitch (+ _returnvalue_yaw 90.0)))
  ; Level Editor Funcitons
  (`SceneComponent.K2_SetWorldRotation` (`self.Cube`) _returnvalue false false)
  (set `self.Origin Rotation` _returnvalue))

(fn `CheckRotationRelationship`
  (params (IsStraightTrack :type Boolean) (TrackRef :type "Actor Object Reference"))
  (bind (_returnvalue_roll _returnvalue_pitch _returnvalue_yaw) (`KismetMathLibrary.BreakRotator` (`self.K2_GetActorRotation` (`self.TrackRef`))))
  (bind (_returnvalue_roll_2 _returnvalue_pitch_2 _returnvalue_yaw_2) (`KismetMathLibrary.BreakRotator` (`self.K2_GetActorRotation` (`self.TrackRef`))))
  ; Checks if Cart can move onto next track based on Cart's and Track's rotations
  (set `self.TrackRef` TrackRef)
  (if IsStraightTrack
    (if (or (== (`SceneComponent.K2_GetComponentRotation` (`self.Cube`)) (`self.K2_GetActorRotation` (`self.TrackRef`)) :`ErrorTolerance` 10.0) (== (`SceneComponent.K2_GetComponentRotation` (`self.Cube`)) (`KismetMathLibrary.MakeRotator` _returnvalue_roll_2 _returnvalue_pitch_2 (+ _returnvalue_yaw_2 180.0)) :`ErrorTolerance` 10.0))
      (bind _asbp_editor_track (cast `/Game/BluePrints/LevelEditorBlueprints/BP_EditorTrack` (`self.TrackRef`)))
      (`self.Move along Straight Path` (`/Game/BluePrints/LevelEditorBlueprints/BP_EditorTrack.MinecartPath` _asbp_editor_track))
      (else
        (`self.Reset Cart`)))
    (elif (or (== (`SceneComponent.K2_GetComponentRotation` (`self.Cube`)) (`self.K2_GetActorRotation` (`self.TrackRef`)) :`ErrorTolerance` 10.0) (== (`SceneComponent.K2_GetComponentRotation` (`self.Cube`)) (`KismetMathLibrary.MakeRotator` _returnvalue_roll _returnvalue_pitch (- _returnvalue_yaw 90.0)) :`ErrorTolerance` 10.0))
      (bind _asbp_editor_turn_track (cast `/Game/BluePrints/LevelEditorBlueprints/BP_EditorTurnTrack` (`self.TrackRef`)))
      (`self.Move Along Turn Track` (`/Game/BluePrints/LevelEditorBlueprints/BP_EditorTurnTrack.MinecartPath` _asbp_editor_turn_track))
      (else
        (`self.Reset Cart`)))))

(fn `UserConstructionScript`
  (`SceneComponent.K2_SetWorldRotation` (`self.Cube`) (`self.K2_GetActorRotation`) false false))