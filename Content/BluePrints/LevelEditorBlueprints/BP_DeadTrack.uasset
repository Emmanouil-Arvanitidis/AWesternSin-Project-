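; BP_DeadTrack is a track tile actor used with the level editor, carrying a track number.
; Editor events set that number and rotate the tile by 90 degrees of yaw per call.
; RotateTrack is an empty event; a Timeline-driven yaw animation that checks for a matching track number and plays or reverses by current yaw is left unconnected, so it never runs.
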(event `self.RotateTrack`
  (params (TrackNumber :type Integer)))

(event `self.ChangeID(Editor)`
  (params (`New ID` :type Integer))
  (set `self.TrackNo` `New ID`))

(event `self.RotateTile(Editor)`
  (bind (_returnvalue_roll _returnvalue_pitch _returnvalue_yaw) (`KismetMathLibrary.BreakRotator` (`self.K2_GetActorRotation`)))
  (`self.K2_SetActorRotation` (`KismetMathLibrary.MakeRotator` _returnvalue_roll _returnvalue_pitch (+ _returnvalue_yaw 90.0))))

(fn `UserConstructionScript`)