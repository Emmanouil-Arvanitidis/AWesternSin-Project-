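; Level editor grid cell that holds a placed straight track, turn track, lever, or minecart with a track beneath it.
; Placing on an empty cell spawns the editor actors at the Arrow's location and stores references to them.
; Placing on an occupied cell instead opens a WB_TileInfo widget showing that piece's ID.
; Removal destroys the stored actors, while rotation and ID changes are forwarded to them as messages.
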(event `/Game/BluePrints/LevelEditorBlueprints/Interfaces/BPI_Grid_Functionality.PlaceTile`
  (params (TileType :type "/Game/BluePrints/LevelEditorBlueprints/Enums/E_TileTypes Enum" :default "NewEnumerator0"))
  ; Places tiles or pulls up HUDWidget
  (`WidgetLayoutLibrary.RemoveAllWidgets`)
  (if (`self.Occupied`)
    (`self.HandleHUDWidget`)
    (else
      (set `self.Occupied` true)
      (`self.SpawnTile` TileType))))

(event `/Game/BluePrints/LevelEditorBlueprints/Interfaces/BPI_Grid_Functionality.RemoveTile`
  (bind _placedtileref (`self.PlacedTileRef`))
  ; Actors controlled by this tile are removed and references are cleared
  (if (`self.Occupied`)
    (`/Engine/EditorBlueprintResources/StandardMacros.IsValid` _placedtileref
      (:`Is Valid`
        (`self.K2_DestroyActor` _placedtileref)
        (set `self.PlacedTileRef` null)
        (if (`self.HasMinecart`)
          (`self.K2_DestroyActor` (`self.MinecartRef`))
          (set `self.HasMinecart` false)
          (set `self.Occupied` false)
          (set `self.MinecartRef` null)
          (`WidgetLayoutLibrary.RemoveAllWidgets`)
          (else
            (set `self.Occupied` false)))))))

(event `/Game/BluePrints/LevelEditorBlueprints/Interfaces/BPI_Grid_Functionality.RotateTile`
  ; Sends RotateTile interface message to controlled tiles
  (message `/Game/BluePrints/LevelEditorBlueprints/Interfaces/BPI_TileFunctionality.RotateTile(Editor)` (`self.PlacedTileRef`))
  (if (`self.HasMinecart`)
    (message `/Game/BluePrints/LevelEditorBlueprints/Interfaces/BPI_TileFunctionality.RotateTile(Editor)` (`self.MinecartRef`))))

(event `/Game/BluePrints/LevelEditorBlueprints/Interfaces/BPI_Grid_Functionality.ChangeTileID`
  (params (`New ID` :type Integer))
  ; Sends ChangeID interface call to controlled tiles
  (if (`self.HasMinecart`)
    (message `/Game/BluePrints/LevelEditorBlueprints/Interfaces/BPI_TileFunctionality.ChangeID(Editor)` (`self.MinecartRef`) `New ID`)
    (else
      (message `/Game/BluePrints/LevelEditorBlueprints/Interfaces/BPI_TileFunctionality.ChangeID(Editor)` (`self.PlacedTileRef`) `New ID`))))

(fn `HandleHUDWidget`
  (bind _placedtileref (`self.PlacedTileRef`))
  ; Creates HUD widget and sends it the correct ID to display
  (bind _returnvalue (`|CreateWidget` "/Game/BluePrints/LevelEditorBlueprints/HUDs/WB_TileInfo.WB_TileInfo_C"))
  (set `/Game/BluePrints/LevelEditorBlueprints/HUDs/WB_TileInfo.SelectedGridTile` self _returnvalue)
  (switch `/Game/BluePrints/LevelEditorBlueprints/Enums/E_TileTypes` (`self.OccupiedTileType`)
    (:`NewEnumerator0`
      (bind _asbp_editor_track (cast `/Game/BluePrints/LevelEditorBlueprints/BP_EditorTrack` _placedtileref))
      (`/Game/BluePrints/LevelEditorBlueprints/HUDs/WB_TileInfo.SetTileIDDisplay` _returnvalue (`/Game/BluePrints/LevelEditorBlueprints/BP_EditorTrack.TrackNo` _asbp_editor_track))
      (`UserWidget.AddToViewport` _returnvalue 0))
    (:`NewEnumerator1`
      (bind _asbp_editor_turn_track (cast `/Game/BluePrints/LevelEditorBlueprints/BP_EditorTurnTrack` _placedtileref))
      (`/Game/BluePrints/LevelEditorBlueprints/HUDs/WB_TileInfo.SetTileIDDisplay` _returnvalue (`/Game/BluePrints/LevelEditorBlueprints/BP_EditorTurnTrack.TurnTrackID` _asbp_editor_turn_track))
      (`UserWidget.AddToViewport` _returnvalue 0))
    (:`NewEnumerator2`
      (bind _asbp_editor_lever (cast `/Game/BluePrints/LevelEditorBlueprints/BP_EditorLever` _placedtileref))
      (`/Game/BluePrints/LevelEditorBlueprints/HUDs/WB_TileInfo.SetTileIDDisplay` _returnvalue (`/Game/BluePrints/LevelEditorBlueprints/BP_EditorLever.LeverNo` _asbp_editor_lever))
      (`UserWidget.AddToViewport` _returnvalue 0))
    (:`NewEnumerator3`
      (bind _asbp_editor_minecart (cast `/Game/BluePrints/LevelEditorBlueprints/BP_EditorMinecart` (`self.MinecartRef`)))
      (`/Game/BluePrints/LevelEditorBlueprints/HUDs/WB_TileInfo.SetTileIDDisplay` _returnvalue (`/Game/BluePrints/LevelEditorBlueprints/BP_EditorMinecart.CartID` _asbp_editor_minecart))
      (`UserWidget.AddToViewport` _returnvalue 0))))

(fn `SpawnTile`
  (params (TileType :type "/Game/BluePrints/LevelEditorBlueprints/Enums/E_TileTypes Enum" :default "NewEnumerator0"))
  ; Spawns correct Actor(s) based on selected TileType
  (switch `/Game/BluePrints/LevelEditorBlueprints/Enums/E_TileTypes` TileType
    (:`NewEnumerator0`
      (bind _returnvalue (`|SpawnActorFromClass` "/Game/BluePrints/LevelEditorBlueprints/BP_EditorTrack.BP_EditorTrack_C" (`KismetMathLibrary.MakeTransform` (`SceneComponent.K2_GetComponentLocation` (`self.Arrow`))) "Undefined" "MultiplyWithRoot" null null))
      (set `self.PlacedTileRef` _returnvalue)
      (set `self.OccupiedTileType` "NewEnumerator0"))
    (:`NewEnumerator1`
      (bind _returnvalue_2 (`|SpawnActorFromClass` "/Game/BluePrints/LevelEditorBlueprints/BP_EditorTurnTrack.BP_EditorTurnTrack_C" (`KismetMathLibrary.MakeTransform` (`SceneComponent.K2_GetComponentLocation` (`self.Arrow`))) "Undefined" "MultiplyWithRoot" null null))
      (set `self.PlacedTileRef` _returnvalue_2)
      (set `self.OccupiedTileType` "NewEnumerator1"))
    (:`NewEnumerator2`
      (bind _returnvalue_3 (`|SpawnActorFromClass` "/Game/BluePrints/LevelEditorBlueprints/BP_EditorLever.BP_EditorLever_C" (`KismetMathLibrary.MakeTransform` (`SceneComponent.K2_GetComponentLocation` (`self.Arrow`))) "Undefined" "MultiplyWithRoot" null null))
      (set `self.PlacedTileRef` _returnvalue_3)
      (set `self.OccupiedTileType` "NewEnumerator2"))
    (:`NewEnumerator3`
      (bind _returnvalue_4 (`|SpawnActorFromClass` "/Game/BluePrints/LevelEditorBlueprints/BP_EditorTrack.BP_EditorTrack_C" (`KismetMathLibrary.MakeTransform` (`SceneComponent.K2_GetComponentLocation` (`self.Arrow`))) "Undefined" "MultiplyWithRoot" null null))
      (set `self.PlacedTileRef` _returnvalue_4)
      (bind _returnvalue_5 (`|SpawnActorFromClass` "/Game/BluePrints/LevelEditorBlueprints/BP_EditorMinecart.BP_EditorMinecart_C" (`KismetMathLibrary.MakeTransform` (`SceneComponent.K2_GetComponentLocation` (`self.Arrow`))) "Undefined" "MultiplyWithRoot" null null))
      (set `self.MinecartRef` _returnvalue_5)
      (set `self.HasMinecart` true)
      (set `self.OccupiedTileType` "NewEnumerator3"))))

(fn `UserConstructionScript`)