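; BP_EditorLever is a level editor lever that triggers track tile rotation by ID.
; PullLever animates the mesh pitch with a timeline, blocks re-pulls until it finishes, and sends RotateTrackMessage with LeverNo once per pull.
; The message goes to every BPI_TileFunctionality actor, since several tiles can share an ID.
; Editor events set LeverNo or yaw the lever in quarter turns, and SetTrackArray caches BPI_LeverFunctionality actors.
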(event `/Game/BluePrints/BlueprintInterfaces/BPI_LeverFunctionality.PullLever`
  ; Plays animation and sends interface message to all actors that implement interface. We cannot send interface message to specific actors as there may be multiple tiles with the correct IDs
  (if (`self.Process`)
    (set `self.Process` false)
    (bind (_direction _newtrack_0) (`Timeline|Timeline` :!via `PlayFromStart`)
      (:`Update`
        (`SceneComponent.K2_SetRelativeRotation` (`self.StaticMesh`) (`KismetMathLibrary.MakeRotator` 0.0 (* _newtrack_0 120.0)) false false)
        (`/Engine/EditorBlueprintResources/StandardMacros.DoOnce` false :!label _label
          (:`Completed`
            (bind _outactors (`GameplayStatics.GetAllActorsWithInterface` "/Game/BluePrints/LevelEditorBlueprints/Interfaces/BPI_TileFunctionality.BPI_TileFunctionality_C"))
            (message `/Game/BluePrints/BlueprintInterfaces/BPI_LeverFunctionality.RotateTrack` _outactors (`self.LeverNo`)))))
      (:`Finished`
        (set `self.Process` true)
        (goto _label :!via `Reset`)))))

(event `/Game/BluePrints/LevelEditorBlueprints/Interfaces/BPI_TileFunctionality.ChangeID(Editor)`
  (params (`New ID` :type Integer))
  (set `self.LeverNo` `New ID`))

(event `/Game/BluePrints/LevelEditorBlueprints/Interfaces/BPI_TileFunctionality.RotateTile(Editor)`
  (bind (_returnvalue_roll _returnvalue_pitch _returnvalue_yaw) (`KismetMathLibrary.BreakRotator` (`self.K2_GetActorRotation`)))
  (`self.K2_SetActorRotation` (`KismetMathLibrary.MakeRotator` _returnvalue_roll _returnvalue_pitch (+ _returnvalue_yaw 90.0))))

(fn `SetTrackArray`
  (bind _outactors (`GameplayStatics.GetAllActorsWithInterface` "/Game/BluePrints/BlueprintInterfaces/BPI_LeverFunctionality.BPI_LeverFunctionality_C"))
  (set `self.TrackArray` _outactors))

(fn `UserConstructionScript`)