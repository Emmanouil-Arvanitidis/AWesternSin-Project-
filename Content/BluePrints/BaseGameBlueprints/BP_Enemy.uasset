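; BP_Enemy is an enemy character that chases the player and triggers a jumpscare death on contact.
; StartChase runs AI MoveTo toward the player character, and EndChase halts its movement immediately; neither is called within this Blueprint.
; Actor overlap passes itself to the player's JumpscareMessage.
; A separate Box overlap with the player plays a 2D scare sound, then opens the DeathMenu level after a short delay.
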(event `self.ReceiveActorBeginOverlap`
  (params (OtherActor :type "Actor Object Reference"))
  (bind _asbp_third_person_character (cast `/Game/ThirdPerson/Blueprints/BP_ThirdPersonCharacter` OtherActor))
  (message `/Game/BluePrints/BlueprintInterfaces/BPI_PlayerInteraction.Jumpscare` _asbp_third_person_character self))

(event `/Game/BluePrints/BlueprintInterfaces/BPI_PlayerInteraction.StartChase`
  (bind _asbp_third_person_character (cast `/Game/ThirdPerson/Blueprints/BP_ThirdPersonCharacter` (`GameplayStatics.GetPlayerCharacter` 0)))
  (`|AIMoveTo` self (0.0 0.0 0.0) _asbp_third_person_character))

(event `/Game/BluePrints/BlueprintInterfaces/BPI_PlayerInteraction.EndChase`
  (`MovementComponent.StopMovementImmediately` (`self.CharacterMovement`)))

(event `self.Box.OnComponentBeginOverlap`
  (params (OverlappedComponent :type "PrimitiveComponent Object Reference") (OtherActor :type "Actor Object Reference") (OtherComp :type "PrimitiveComponent Object Reference") (OtherBodyIndex :type Integer) (bFromSweep :type Boolean) (SweepResult :type "HitResult Structure (by ref)"))
  (cast `/Game/ThirdPerson/Blueprints/BP_ThirdPersonCharacter` OtherActor)
  (`GameplayStatics.PlaySound2D` "/Game/SFX/Jumpscare/712416__zombyklr__jumpscare-1.712416__zombyklr__jumpscare-1" 1.0 1.0 0.0 null null)
  (`KismetSystemLibrary.Delay` 1.0)
  (`GameplayStatics.OpenLevelBySoftObjectPtr` "/Game/UIElements/Menus/DeathMenu/DeathMenu.DeathMenu"))

(fn `UserConstructionScript`)