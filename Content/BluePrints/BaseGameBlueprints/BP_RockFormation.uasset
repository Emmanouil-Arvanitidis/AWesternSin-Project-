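; BP_RockFormation is a rock formation actor that moves vertically the first time something overlaps it.
; The overlap toggles its particle system's visibility unless the actor has the "Nodust" tag, then plays a timeline.
; Each timeline update adds the track value to the root's current world Z and sets it as relative location, so offsets accumulate.
; When the timeline finishes, the particle component is destroyed after a short delay.
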(event `self.ReceiveActorBeginOverlap`
  (params (OtherActor :type "Actor Object Reference"))
  (bind (_returnvalue_x _returnvalue_y _returnvalue_z) (`KismetMathLibrary.BreakVector` (`SceneComponent.K2_GetComponentLocation` (`self.DefaultSceneRoot`))))
  (`/Engine/EditorBlueprintResources/StandardMacros.DoOnce` false
    (:`Completed`
      (if (`self.ActorHasTag` "Nodust")
        (bind (_direction _newtrack_0) (`Timeline|Timeline` :!label _label)
          (:`Update`
            (`self.K2_SetActorRelativeLocation` (`KismetMathLibrary.MakeVector` _returnvalue_x _returnvalue_y (+ _returnvalue_z _newtrack_0))))
          (:`Finished`
            (`KismetSystemLibrary.Delay` 1.0)
            (`ActorComponent.K2_DestroyComponent` (`self.ParticleSystem`))))
        (else
          (`SceneComponent.ToggleVisibility` (`self.ParticleSystem`) false)
          (goto _label))))))

(fn `UserConstructionScript`)