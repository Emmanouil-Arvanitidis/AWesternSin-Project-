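; BP_ExplotionBeams is a beam structure that explodes when an actor implementing BPI_CartExplode, likely a cart, overlaps it.
; The overlap activates a particle system, then after a short delay sends ExplodeMessage with its ID to the first actor found implementing that interface.
; It then destroys the overlapping actor and removes its own mesh and cube components, leaving the Blueprint actor itself in place.
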(event `self.ReceiveActorBeginOverlap`
  (params (OtherActor :type "Actor Object Reference"))
  (if (`KismetSystemLibrary.DoesImplementInterface` OtherActor "/Game/BluePrints/BlueprintInterfaces/BPI_CartExplode.BPI_CartExplode_C")
    (`ActorComponent.Activate` (`self.ParticleSystem`) false)
    (`KismetSystemLibrary.Delay` 0.1)
    (bind _outactors (`GameplayStatics.GetAllActorsWithInterface` "/Game/BluePrints/BlueprintInterfaces/BPI_CartExplode.BPI_CartExplode_C"))
    (message `/Game/BluePrints/BlueprintInterfaces/BPI_CartExplode.Explode` (`|GetArrayItem` _outactors) (`self.ID`))
    (`self.K2_DestroyActor` OtherActor)
    (`ActorComponent.K2_DestroyComponent` (`self.StaticMesh2`))
    (`ActorComponent.K2_DestroyComponent` (`self.StaticMesh`))
    (`ActorComponent.K2_DestroyComponent` (`self.StaticMesh1`))
    (`ActorComponent.K2_DestroyComponent` (`self.StaticMesh3`))
    (`ActorComponent.K2_DestroyComponent` (`self.Cube`))))

(fn `UserConstructionScript`)