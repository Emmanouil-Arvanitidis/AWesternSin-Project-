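; BP_Lever is a pullable lever that signals track rotation to other actors, identified by its lever number.
; PullLever plays a timeline that pitches the static mesh, with a Process flag blocking repeat pulls until it finishes.
; A DoOnce on the timeline's first update sends RotateTrackMessage with LeverNo to actors implementing BPI_LeverFunctionality, then resets on finish.
; An UpdateArrayMessage call is left unconnected.
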(event `/Game/BluePrints/BlueprintInterfaces/BPI_LeverFunctionality.PullLever`
  (if (`self.Process`)
    (set `self.Process` false)
    (bind (_direction _newtrack_0) (`Timeline|Timeline` :!via `PlayFromStart`)
      (:`Update`
        (`SceneComponent.K2_SetRelativeRotation` (`self.StaticMesh`) (`KismetMathLibrary.MakeRotator` 0.0 (* _newtrack_0 120.0)) false false)
        (`/Engine/EditorBlueprintResources/StandardMacros.DoOnce` false :!label _label
          (:`Completed`
            (bind _outactors (`GameplayStatics.GetAllActorsWithInterface` "/Game/BluePrints/BlueprintInterfaces/BPI_LeverFunctionality.BPI_LeverFunctionality_C"))
            (message `/Game/BluePrints/BlueprintInterfaces/BPI_LeverFunctionality.RotateTrack` _outactors (`self.LeverNo`)))))
      (:`Finished`
        (set `self.Process` true)
        (goto _label :!via `Reset`)))))

(fn `UserConstructionScript`)