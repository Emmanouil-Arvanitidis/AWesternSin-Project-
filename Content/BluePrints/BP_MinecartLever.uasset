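; Minecart lever that animates when pulled and signals carts to start.
; PullLever uses the Triggered flag to block re-entry while a Timeline pitches the lever mesh.
; On every Timeline update, not just once, it finds all BPI_LeverFunctionality actors and sends them StartCartMessage with its LeverID.
; The flag resets when the Timeline finishes.
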(event `self.PullLever`
  (`GameplayStatics.GetAllActorsWithInterface` "/Game/BluePrints/BlueprintInterfaces/BPI_LeverFunctionality.BPI_LeverFunctionality_C")
  (if (`self.Triggered`)
    (set `self.Triggered` false)
    (bind (_direction _newtrack_0) (`Timeline|Timeline` :!via `PlayFromStart`)
      (:`Update`
        (`SceneComponent.K2_SetRelativeRotation` (`self.StaticMesh`) (`KismetMathLibrary.MakeRotator` 0.0 (* _newtrack_0 120.0)) false false)
        (bind _outactors (`GameplayStatics.GetAllActorsWithInterface` "/Game/BluePrints/BlueprintInterfaces/BPI_LeverFunctionality.BPI_LeverFunctionality_C"))
        (message `/Game/BluePrints/BlueprintInterfaces/BPI_LeverFunctionality.StartCart` _outactors (`self.LeverID`)))
      (:`Finished`
        (set `self.Triggered` true)))))

(fn `UserConstructionScript`)