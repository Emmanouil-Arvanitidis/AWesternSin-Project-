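; BP_TurnTrack is a track piece that rotates in yaw when a RotateTurnTrack event carries an ID matching its TurnTrackID.
; A timeline played from the start drives the turn, adding its track value to the stored CurrentRotation each update.
; CurrentRotation is captured at BeginPlay and again when the timeline finishes, so each turn builds on the previous one.
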(event `self.ReceiveBeginPlay`
  (bind (_returnvalue_roll _returnvalue_pitch _returnvalue_yaw) (`KismetMathLibrary.BreakRotator` (`self.K2_GetActorRotation`)))
  (set `self.CurrentRotation` _returnvalue_yaw))

(event `/Game/BluePrints/BlueprintInterfaces/BPI_LeverFunctionality.RotateTurnTrack`
  (params (ID :type Integer))
  (bind (_returnvalue_roll _returnvalue_pitch _returnvalue_yaw) (`KismetMathLibrary.BreakRotator` (`self.K2_GetActorRotation`)))
  (if (== ID (`self.TurnTrackID`))
    (bind (_direction _newtrack_0) (`Timeline|Timeline` :!via `PlayFromStart`)
      (:`Update`
        (`self.K2_SetActorRotation` (`KismetMathLibrary.MakeRotator` 0.0 0.0 (+ _newtrack_0 (`self.CurrentRotation`)))))
      (:`Finished`
        (set `self.CurrentRotation` _returnvalue_yaw)))))

(fn `UserConstructionScript`)