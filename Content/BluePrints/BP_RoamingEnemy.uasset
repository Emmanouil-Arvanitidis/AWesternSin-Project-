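; Roaming enemy that wanders random points, chases players carrying a light, and jumpscares them on contact.
; A self-restarting AI MoveTo loop drives roaming, while PawnSensing starts a chase when the seen pawn implements BPI_RoamingFunctionality and has the LIGHTON tag.
; Actor overlap sends the player a jumpscare message and calls StopChase, which resumes roaming only if not chasing.
; Box overlap plays a scare sound, then opens the death menu level.
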(event `self.ReceiveBeginPlay`
  ; Starts Roam Loop
  (`self.Roam`))

(event `self.ReceiveActorBeginOverlap`
  (params (OtherActor :type "Actor Object Reference"))
  ; Jumpscares Player on overlap
  (bind _asbp_third_person_character (cast `/Game/ThirdPerson/Blueprints/BP_ThirdPersonCharacter` OtherActor))
  (`|ExecutionSequence`
    (:`then_0`
      (message `/Game/BluePrints/BlueprintInterfaces/BPI_PlayerInteraction.Jumpscare` _asbp_third_person_character self))
    (:`then_1`
      (`self.StopChase`))))

(event `Chase Player`
  ; Moves towards player
  (set `self.IsChasing` true)
  (bind _asbp_third_person_character (cast `/Game/ThirdPerson/Blueprints/BP_ThirdPersonCharacter` (`GameplayStatics.GetPlayerCharacter` 0)))
  (bind _output_get (set `self.As BP Third Person Character` _asbp_third_person_character))
  (`|AIMoveTo` self (0.0 0.0 0.0) _output_get))

(event `Roam`
  ; Random Roam Loop
  (`|AIMoveTo` self (`KismetMathLibrary.MakeVector` (`KismetMathLibrary.Conv_IntToDouble` (`KismetMathLibrary.RandomIntegerInRange` 1800 6800)) (`KismetMathLibrary.Conv_IntToDouble` (`KismetMathLibrary.RandomIntegerInRange` 5100 8000))) null
    (:`OnSuccess`
      _)
    (:`OnFail`
      _))
  (`KismetSystemLibrary.Delay` 2.0)
  (`self.Roam`))

(event `self.PawnSensing.OnSeePawn`
  (params (Pawn :type "Pawn Object Reference"))
  ; Chase player if their Light is on
  (if (`KismetSystemLibrary.DoesImplementInterface` Pawn "/Game/BluePrints/BlueprintInterfaces/BPI_RoamingFunctionality.BPI_RoamingFunctionality_C")
    (if (`self.ActorHasTag` Pawn "LIGHTON")
      (`self.Chase Player`))))

(event `self.StopChase`
  (if (not (`self.IsChasing`))
    (set `self.IsChasing` false)
    (`self.Roam`)))

(event `self.Box.OnComponentBeginOverlap`
  (params (OverlappedComponent :type "PrimitiveComponent Object Reference") (OtherActor :type "Actor Object Reference") (OtherComp :type "PrimitiveComponent Object Reference") (OtherBodyIndex :type Integer) (bFromSweep :type Boolean) (SweepResult :type "HitResult Structure (by ref)"))
  (cast `/Game/ThirdPerson/Blueprints/BP_ThirdPersonCharacter` OtherActor)
  (`GameplayStatics.PlaySound2D` "/Game/SFX/Jumpscare/712416__zombyklr__jumpscare-1.712416__zombyklr__jumpscare-1" 1.0 1.0 0.0 null null)
  (`KismetSystemLibrary.Delay` 1.0)
  (`GameplayStatics.OpenLevelBySoftObjectPtr` "/Game/UIElements/Menus/DeathMenu/DeathMenu.DeathMenu"))

(fn `UserConstructionScript`)