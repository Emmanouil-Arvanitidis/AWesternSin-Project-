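; Minecart that, when StartCart matches its CartID, rides along track pieces from a game jam puzzle.
; MoveCart recurses each tick, stepping along a BP_MovableTrack aligned with the cart's yaw or snapping 90 degrees through a BP_TurnTrack.
; A track at the wrong rotation sends the cart back to its starting transform after a delay.
; Overlapping BP_ExplotionBeams only plays an explosion sound; BP_EditorMinecart holds an improved version of this logic.
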(event `self.ReceiveBeginPlay`
  (set `self.Origin Location` (`SceneComponent.K2_GetComponentLocation` (`self.Cube`)))
  (set `self.Origin Rotation` (`SceneComponent.K2_GetComponentRotation` (`self.Cube`))))

(event `/Game/BluePrints/BlueprintInterfaces/BPI_LeverFunctionality.StartCart`
  (params (ID :type Integer))
  (if (== ID (`self.CartID`))
    (`self.MoveCart`)))

(event `Reset Cart`
  (`KismetSystemLibrary.Delay` 1.0)
  (`SceneComponent.K2_SetWorldLocationAndRotation` (`self.Cube`) (`self.Origin Location`) (`self.Origin Rotation`) false false))

(event `self.Box.OnComponentBeginOverlap`
  (params (OverlappedComponent :type "PrimitiveComponent Object Reference") (OtherActor :type "Actor Object Reference") (OtherComp :type "PrimitiveComponent Object Reference") (OtherBodyIndex :type Integer) (bFromSweep :type Boolean) (SweepResult :type "HitResult Structure (by ref)"))
  (cast `/Game/BluePrints/BaseGameBlueprints/BP_ExplotionBeams` OtherActor)
  (`GameplayStatics.PlaySound2D` "/Game/TemplateFolders/StarterContent/Audio/Explosion01.Explosion01" 1.0 1.0 0.0 null null))

(event `MoveCart`
  (bind _returnvalue (`SceneComponent.K2_GetComponentRotation` (`self.Cube`)))
  (bind (_returnvalue_roll _returnvalue_pitch _returnvalue_yaw) (`KismetMathLibrary.BreakRotator` (`SceneComponent.K2_GetComponentRotation` (`self.Cube`))))
  (bind (_returnvalue_x _returnvalue_y _returnvalue_z) (`KismetMathLibrary.BreakVector` (`SceneComponent.K2_GetComponentLocation` (`self.Cube`))))
  (bind (_returnvalue_roll_2 _returnvalue_pitch_2 _returnvalue_yaw_2) (`KismetMathLibrary.BreakRotator` (`SceneComponent.K2_GetComponentRotation` (`self.Cube`))))
  (bind (_returnvalue_x_2 _returnvalue_y_2 _returnvalue_z_2) (`KismetMathLibrary.BreakVector` (`SceneComponent.K2_GetComponentLocation` (`self.Cube`))))
  (bind _returnvalue_2 (`SceneComponent.K2_GetComponentRotation` (`self.Cube`)))
  (bind (_returnvalue_roll_3 _returnvalue_pitch_3 _returnvalue_yaw_3) (`KismetMathLibrary.BreakRotator` (`SceneComponent.K2_GetComponentRotation` (`self.Cube`))))
  (bind (_returnvalue_x_3 _returnvalue_y_3 _returnvalue_z_3) (`KismetMathLibrary.BreakVector` (`SceneComponent.K2_GetComponentLocation` (`self.Cube`))))
  (bind (_returnvalue_roll_4 _returnvalue_pitch_4 _returnvalue_yaw_4) (`KismetMathLibrary.BreakRotator` (`SceneComponent.K2_GetComponentRotation` (`self.Cube`))))
  (bind (_returnvalue_x_4 _returnvalue_y_4 _returnvalue_z_4) (`KismetMathLibrary.BreakVector` (`SceneComponent.K2_GetComponentLocation` (`self.Cube`))))
  (bind (_returnvalue_roll_5 _returnvalue_pitch_5 _returnvalue_yaw_5) (`KismetMathLibrary.BreakRotator` (`SceneComponent.K2_GetComponentRotation` (`self.Cube`))))
  (bind (_returnvalue_x_5 _returnvalue_y_5 _returnvalue_z_5) (`KismetMathLibrary.BreakVector` (`SceneComponent.K2_GetComponentLocation` (`self.Cube`))))
  (bind (_returnvalue_roll_6 _returnvalue_pitch_6 _returnvalue_yaw_6) (`KismetMathLibrary.BreakRotator` (`SceneComponent.K2_GetComponentRotation` (`self.Cube`))))
  (bind (_returnvalue_x_6 _returnvalue_y_6 _returnvalue_z_6) (`KismetMathLibrary.BreakVector` (`SceneComponent.K2_GetComponentLocation` (`self.Cube`))))
  (bind (_returnvalue_roll_7 _returnvalue_pitch_7 _returnvalue_yaw_7) (`KismetMathLibrary.BreakRotator` (`SceneComponent.K2_GetComponentRotation` (`self.Cube`))))
  (bind (_returnvalue_x_7 _returnvalue_y_7 _returnvalue_z_7) (`KismetMathLibrary.BreakVector` (`SceneComponent.K2_GetComponentLocation` (`self.Cube`))))
  (bind (_returnvalue_roll_8 _returnvalue_pitch_8 _returnvalue_yaw_8) (`KismetMathLibrary.BreakRotator` (`SceneComponent.K2_GetComponentRotation` (`self.Cube`))))
  (bind (_returnvalue_x_8 _returnvalue_y_8 _returnvalue_z_8) (`KismetMathLibrary.BreakVector` (`SceneComponent.K2_GetComponentLocation` (`self.Cube`))))
  (bind _output (`|GetArrayItem` (`PrimitiveComponent.GetOverlappingActors` (`self.Box`) "/Game/BluePrints/BP_TurnTrack.BP_TurnTrack_C")))
  (bind _output_2 (`|GetArrayItem` (`PrimitiveComponent.GetOverlappingActors` (`self.Box`) "/Game/BluePrints/BP_MovableTrack.BP_MovableTrack_C")))
  (bind (_returnvalue_roll_9 _returnvalue_pitch_9 _returnvalue_yaw_9) (`KismetMathLibrary.BreakRotator` (`self.K2_GetActorRotation` _output)))
  (bind (_returnvalue_roll_10 _returnvalue_pitch_10 _returnvalue_yaw_10) (`KismetMathLibrary.BreakRotator` (`self.K2_GetActorRotation` _output)))
  (bind (_returnvalue_roll_11 _returnvalue_pitch_11 _returnvalue_yaw_11) (`KismetMathLibrary.BreakRotator` (`self.K2_GetActorRotation` _output_2)))
  (bind (_returnvalue_roll_12 _returnvalue_pitch_12 _returnvalue_yaw_12) (`KismetMathLibrary.BreakRotator` (`self.K2_GetActorRotation` _output)))
  (bind (_returnvalue_roll_13 _returnvalue_pitch_13 _returnvalue_yaw_13) (`KismetMathLibrary.BreakRotator` (`self.K2_GetActorRotation` _output)))
  (bind (_returnvalue_roll_14 _returnvalue_pitch_14 _returnvalue_yaw_14) (`KismetMathLibrary.BreakRotator` (`self.K2_GetActorRotation` _output)))
  (bind _returnvalue_3 (`self.IsOverlappingActor` _output_2))
  (bind (_returnvalue_roll_15 _returnvalue_pitch_15 _returnvalue_yaw_15) (`KismetMathLibrary.BreakRotator` (`self.K2_GetActorRotation` _output)))
  (bind (_returnvalue_roll_16 _returnvalue_pitch_16 _returnvalue_yaw_16) (`KismetMathLibrary.BreakRotator` (`self.K2_GetActorRotation` _output)))
  (bind (_returnvalue_roll_17 _returnvalue_pitch_17 _returnvalue_yaw_17) (`KismetMathLibrary.BreakRotator` (`self.K2_GetActorRotation` _output)))
  ;[1 1 1] Logic for which way the cart will move according to its rotation and the rotation of the track (recuring).    This code has been improved and made more efficient on the Level Editor Version of this blueprint (All > Content > Blueprints > LevelEditorBlueprints > BP_EditorMinecart ) (I did not want to change this code as I wanted to keep the game jam code the same)
  (if (or _returnvalue_3 (`self.IsOverlappingActor` _output))
    (if _returnvalue_3
      (if (or (== _returnvalue_2 (struct)) (== _returnvalue_2 (struct :`Yaw` 180.0)))
        (if (or (== _returnvalue_yaw_11 0.0) (== _returnvalue_yaw_11 180.0))
          (if (== (`SceneComponent.K2_GetComponentRotation` (`self.Cube`)) (struct))
            (`SceneComponent.K2_SetWorldLocation` (`self.Cube`) (+ (`SceneComponent.K2_GetComponentLocation` (`self.Cube`)) (10.0 0.0 0.0)) false false)
            (else
              (`SceneComponent.K2_SetWorldLocation` (`self.Cube`) (+ (`SceneComponent.K2_GetComponentLocation` (`self.Cube`)) (-10.0 0.0 0.0)) false false)))
          (`KismetSystemLibrary.DelayUntilNextTick` :!label _label)
          (`self.MoveCart`)
          (else
            (`self.Reset Cart`)))
        (elif (or (== _returnvalue (struct :`Yaw` 90.0)) (== _returnvalue (struct :`Yaw` -90.0)))
          (if (or (== _returnvalue_yaw_11 90.0) (== -90.0 _returnvalue_yaw_11))
            (if (== (`SceneComponent.K2_GetComponentRotation` (`self.Cube`)) (struct :`Yaw` 90.0) :`ErrorTolerance` 10.0)
              (`SceneComponent.K2_SetWorldLocation` (`self.Cube`) (+ (`SceneComponent.K2_GetComponentLocation` (`self.Cube`)) (0.0 10.0 0.0)) false false)
              (goto _label)
              (else
                (`SceneComponent.K2_SetWorldLocation` (`self.Cube`) (- (`SceneComponent.K2_GetComponentLocation` (`self.Cube`)) (0.0 10.0 0.0)) false false)
                (goto _label)))
            (else
              (`self.Reset Cart`)))))
      (elif (== (`SceneComponent.K2_GetComponentRotation` (`self.Cube`)) (struct))
        (if (== _returnvalue_yaw_13 0.0)
          (`SceneComponent.K2_SetWorldRotation` (`self.Cube`) (`KismetMathLibrary.MakeRotator` _returnvalue_roll_5 _returnvalue_pitch_5 (+ _returnvalue_yaw_5 90.0)) false false)
          (`SceneComponent.K2_SetWorldLocation` (`self.Cube`) (`KismetMathLibrary.MakeVector` (+ _returnvalue_x_5 80.0) (+ _returnvalue_y_5 150.0) _returnvalue_z_5) false false)
          (goto _label)
          (elif (== _returnvalue_yaw_14 90.0)
            (`SceneComponent.K2_SetWorldRotation` (`self.Cube`) (`KismetMathLibrary.MakeRotator` _returnvalue_roll_3 _returnvalue_pitch_3 (- _returnvalue_yaw_3 90.0)) false false)
            (`SceneComponent.K2_SetWorldLocation` (`self.Cube`) (`KismetMathLibrary.MakeVector` (+ _returnvalue_x_3 80.0) (- _returnvalue_y_3 150.0) _returnvalue_z_3) false false)
            (goto _label)
            (else
              (`self.Reset Cart`))))
        (elif (== (`SceneComponent.K2_GetComponentRotation` (`self.Cube`)) (struct :`Yaw` 90.0))
          (if (== _returnvalue_yaw_16 180.0)
            (`SceneComponent.K2_SetWorldRotation` (`self.Cube`) (`KismetMathLibrary.MakeRotator` _returnvalue_roll_7 _returnvalue_pitch_7 (- _returnvalue_yaw_7 90.0)) false false)
            (`SceneComponent.K2_SetWorldLocation` (`self.Cube`) (`KismetMathLibrary.MakeVector` (+ _returnvalue_x_7 150.0) (+ _returnvalue_y_7 80.0) _returnvalue_z_7) false false)
            (goto _label)
            (elif (== _returnvalue_yaw_17 90.0)
              (`SceneComponent.K2_SetWorldRotation` (`self.Cube`) (`KismetMathLibrary.MakeRotator` _returnvalue_roll_4 _returnvalue_pitch_4 (+ _returnvalue_yaw_4 90.0)) false false)
              (`SceneComponent.K2_SetWorldLocation` (`self.Cube`) (`KismetMathLibrary.MakeVector` (- _returnvalue_x_4 150.0) (+ _returnvalue_y_4 80.0) _returnvalue_z_4) false false)
              (goto _label)
              (else
                (`self.Reset Cart`))))
          (elif (== (`SceneComponent.K2_GetComponentRotation` (`self.Cube`)) (struct :`Yaw` 180.0))
            (if (== _returnvalue_yaw_9 180.0)
              (`SceneComponent.K2_SetWorldRotation` (`self.Cube`) (`KismetMathLibrary.MakeRotator` _returnvalue_roll_2 _returnvalue_pitch_2 (+ _returnvalue_yaw_2 90.0)) false false)
              (`SceneComponent.K2_SetWorldLocation` (`self.Cube`) (`KismetMathLibrary.MakeVector` (- _returnvalue_x_2 80.0) (- _returnvalue_y_2 150.0) _returnvalue_z_2) false false)
              (goto _label)
              (elif (== _returnvalue_yaw_10 -90.0)
                (`SceneComponent.K2_SetWorldRotation` (`self.Cube`) (`KismetMathLibrary.MakeRotator` _returnvalue_roll _returnvalue_pitch (- _returnvalue_yaw 90.0)) false false)
                (`SceneComponent.K2_SetWorldLocation` (`self.Cube`) (`KismetMathLibrary.MakeVector` (- _returnvalue_x 80.0) (+ _returnvalue_y 150.0) _returnvalue_z) false false)
                (goto _label)
                (else
                  (`self.Reset Cart`))))
            (elif (== (`SceneComponent.K2_GetComponentRotation` (`self.Cube`)) (struct :`Yaw` -90.0))
              (if (== _returnvalue_yaw_12 0.0)
                (`SceneComponent.K2_SetWorldRotation` (`self.Cube`) (`KismetMathLibrary.MakeRotator` _returnvalue_roll_6 _returnvalue_pitch_6 (- _returnvalue_yaw_6 90.0)) false false)
                (`SceneComponent.K2_SetWorldLocation` (`self.Cube`) (`KismetMathLibrary.MakeVector` (- _returnvalue_x_6 150.0) (- _returnvalue_y_6 80.0) _returnvalue_z_6) false false)
                (goto _label)
                (elif (== _returnvalue_yaw_15 -90.0)
                  (`SceneComponent.K2_SetWorldRotation` (`self.Cube`) (`KismetMathLibrary.MakeRotator` _returnvalue_roll_8 _returnvalue_pitch_8 (+ _returnvalue_yaw_8 90.0)) false false)
                  (`SceneComponent.K2_SetWorldLocation` (`self.Cube`) (`KismetMathLibrary.MakeVector` (+ _returnvalue_x_8 150.0) (- _returnvalue_y_8 80.0) _returnvalue_z_8) false false)
                  (goto _label)
                  (else
                    (`self.Reset Cart`)))))))))))

(fn `UserConstructionScript`
  (`SceneComponent.K2_SetWorldRotation` (`self.Cube`) (`self.K2_GetActorRotation`) false false))